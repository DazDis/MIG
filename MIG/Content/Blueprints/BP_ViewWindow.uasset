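; BP_ViewWindow is an actor that displays text through a UI_ViewWindow widget held in its UIViewWindow component.
; On BeginPlay it caches the cast widget and passes CurrentText to EnterMainText; the SetText call that follows is an empty stub.
; ChangeVisibility acts only when the requested state differs, toggling the Plane component and propagating the change to its children.
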(event `self.ReceiveBeginPlay`
  (`parent.ReceiveBeginPlay`)
  (`self.InitVariables`)
  (`self.Set text`))

(fn `ChangeVisibility`
  (params (Visibility :type Boolean))
  (if (!= Visibility (`self.Visible`))
    (bind _output_get (set `self.Visible` (not (`self.Visible`))))
    (`SceneComponent.SetVisibility` (`self.Plane`) _output_get true)))

(fn `InitVariables`
  (bind _asui_view_window (cast `/Game/Blueprints/UI_ViewWindow` (`WidgetComponent.GetWidget` (`self.UI_ViewWindow`))))
  (set `self.UI_ViewWindowInfo` _asui_view_window)
  (`/Game/Blueprints/UI_ViewWindow.EnterMainText` (`self.UI_ViewWindowInfo`) (`self.CurrentText`)))

(fn `Set text`)

(fn `UserConstructionScript`)