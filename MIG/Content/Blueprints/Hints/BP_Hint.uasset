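; BP_Hint is a hint actor that displays configurable text and can briefly reveal a cube when its trigger is overlapped.
; On BeginPlay, it copies TextOfHint into the TextRender component.
; When Trigger begins an overlap and ShowSquare is false, it shows Cube and its children, then hides them after a HintTime delay.
; The overlap does not filter which actor entered.
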(event `self.ReceiveBeginPlay`
  (`TextRenderComponent.K2_SetText` (`self.TextRender`) (`self.TextOfHint`)))

(event `self.Trigger.OnComponentBeginOverlap`
  (params (OverlappedComponent :type "PrimitiveComponent Object Reference") (OtherActor :type "Actor Object Reference") (OtherComp :type "PrimitiveComponent Object Reference") (OtherBodyIndex :type Integer) (bFromSweep :type Boolean) (SweepResult :type "HitResult Structure (by ref)"))
  (if (not (`self.Show_Square`))
    (`SceneComponent.SetVisibility` (`self.Cube`) true true)
    (`KismetSystemLibrary.Delay` (`self.HintTime`))
    (`SceneComponent.SetVisibility` (`self.Cube`) false true)))

(fn `UserConstructionScript`)