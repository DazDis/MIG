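; Trigger box that makes an overlapping BP_Unkers fire a two-shot burst of BP_Projectile from its GunCenter.
; Overlaps by projectiles are ignored; any other actor starts the sequence and cooldown, though only BP_Unkers fires.
; The NotActivated gate closes only after the short delay between shots, then reopens after a cooldown.
; ChangeSpeedOfJet, which scales a parent BP_MIG's JetSpeed, is defined but not called here.
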(event `self.ReceiveActorBeginOverlap`
  (params (OtherActor :type "Actor Object Reference"))
  (if (== (`GameplayStatics.GetObjectClass` OtherActor) "/Game/Blueprints/Waypoint_System/BP_Projectile.BP_Projectile_C")
    _
    (elif (`self.NotActivated`)
      (`self.StartFiring` OtherActor)
      (`KismetSystemLibrary.Delay` 0.2)
      (`self.StartFiring` OtherActor)
      (set `self.NotActivated` false)
      (`KismetSystemLibrary.Delay` 3.0)
      (set `self.NotActivated` true))))

(fn `ChangeSpeedOfJet`
  (params (`In Actor` :type "Actor Object Reference") (Multiplier :type "Float (double-precision)"))
  (bind _asbp_mig (cast `/Game/Blueprints/BP_MIG` (`self.GetParentActor` `In Actor`)))
  (set `/Game/Blueprints/BP_MIG.JetSpeed` (* (`/Game/Blueprints/BP_MIG.JetSpeed` _asbp_mig) Multiplier) _asbp_mig)
  (set `self.NotActivated` false))

(fn `StartFiring`
  (params (`In Actor` :type "Actor Object Reference"))
  (bind _asbp_unkers (cast `/Game/Blueprints/BP_Unkers` `In Actor`))
  (bind _guncenter (`/Game/Blueprints/BP_Unkers.GunCenter` _asbp_unkers))
  (`|SpawnActorFromClass` "/Game/Blueprints/Waypoint_System/BP_Projectile.BP_Projectile_C" (`KismetMathLibrary.MakeTransform` (`SceneComponent.K2_GetComponentLocation` _guncenter) (`SceneComponent.K2_GetComponentRotation` _guncenter)) "Undefined" "MultiplyWithRoot" null null))

(fn `UserConstructionScript`)