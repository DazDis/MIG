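; Trigger box that gradually slows an overlapping BP_Unkers jet toward a target speed.
; On overlap, a Delay-driven loop subtracts SpeedAddInTick from JetSpeed every TickInterval while it exceeds SpeedToSet.
; The NotActivated flag gates re-entry and is restored by a three-second delay, though each slowdown step clears it again.
; A debug "Hello" prints on activation.
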(event `self.ReceiveActorBeginOverlap`
  (params (OtherActor :type "Actor Object Reference"))
  (`|ExecutionSequence`
    (:`then_0`
      (if (`self.NotActivated`)
        (set `self.NotActivated` false)
        (bind _asbp_unkers (cast `/Game/Blueprints/BP_Unkers` OtherActor)
          (:`then`
            _)
          (:`CastFailed`
            _))
        (`KismetSystemLibrary.PrintString` "Hello")
        (if (> (`/Game/Blueprints/BP_Unkers.JetSpeed` _asbp_unkers) (`self.Speed To Set`)) :!label _label
          (`KismetSystemLibrary.Delay` (`self.TickInterval`))
          (`self.ChangeSpeedOfJet` OtherActor :!pinned true) ; Изменяет скорость самолета на множитель Multiplier\nДля работы подсоединить свойство Other Actor к In Actor
          (goto _label))))
    (:`then_1`
      (`KismetSystemLibrary.Delay` 3.0)
      (set `self.NotActivated` true))))

(fn `ChangeSpeedOfJet`
  (params (`In Actor` :type "Actor Object Reference"))
  (bind _asbp_unkers (cast `/Game/Blueprints/BP_Unkers` `In Actor`))
  (set `/Game/Blueprints/BP_Unkers.JetSpeed` (- (`/Game/Blueprints/BP_Unkers.JetSpeed` _asbp_unkers) (`self.SpeedAddInTick`)) _asbp_unkers)
  (set `self.NotActivated` false))

(fn `UserConstructionScript`)