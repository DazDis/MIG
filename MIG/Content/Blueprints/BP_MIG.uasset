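; MIG aircraft actor that plays a timed sequence of informational tip windows.
; On BeginPlay it caches four BP_ViewWindow child actors as start, first, second and end tips, leaving only the start tip unhidden.
; StartTips fades in the idle audio and runs the Tips timeline, whose tracks toggle the middle windows.
; On finish it shows the end tip and sets FlyInProcess, which blocks any replay.
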(event `self.ReceiveBeginPlay`
  (`self.InitVariables`))

(event `Event StartTips`
  (if (`KismetMathLibrary.BooleanNOR` (`self.TipsIsGoing`) (`self.FlyInProcess`))
    (`AudioComponent.FadeIn` (`self.MIG_idle`) 2.0 1.0 0.0 "Linear")
    (set `self.TipsIsGoing` true)
    (bind (_direction _tip _tip2) (`Timeline|Tips` :!via `PlayFromStart`)
      (:`Update`
        (`/Game/Blueprints/BP_ViewWindow.ChangeVisibility` (`self.StartTip`) false)
        (`/Game/Blueprints/BP_ViewWindow.ChangeVisibility` (`self.FirstTip`) (>= _tip 1.0))
        (`/Game/Blueprints/BP_ViewWindow.ChangeVisibility` (`self.SecondTip`) (>= _tip2 1.0)))
      (:`Finished`
        (`/Game/Blueprints/BP_ViewWindow.ChangeVisibility` (`self.EndTip`) true)
        (set `self.TipsIsGoing` false)
        (set `self.FlyInProcess` true)))))

(event `self.ReceiveTick`
  (params (DeltaSeconds :type "Float (single-precision)")))

(fn `InitVariables`
  (`|ExecutionSequence`
    (:`then_0`
      (bind _asbp_view_window (cast `/Game/Blueprints/BP_ViewWindow` (`ChildActorComponent.ChildActor` (`self.BP_ViewWindow`))))
      (bind _output_get (set `self.FirstTip` _asbp_view_window))
      (`/Game/Blueprints/BP_ViewWindow.ChangeVisibility` _output_get false)
      (bind _asbp_view_window_2 (cast `/Game/Blueprints/BP_ViewWindow` (`ChildActorComponent.ChildActor` (`self.BP_ViewWindow1`))))
      (bind _output_get_2 (set `self.SecondTip` _asbp_view_window_2))
      (`/Game/Blueprints/BP_ViewWindow.ChangeVisibility` _output_get_2 false)
      (bind _asbp_view_window_3 (cast `/Game/Blueprints/BP_ViewWindow` (`ChildActorComponent.ChildActor` (`self.BP_ViewWindow2`))))
      (set `self.StartTip` _asbp_view_window_3)
      (bind _asbp_view_window_4 (cast `/Game/Blueprints/BP_ViewWindow` (`ChildActorComponent.ChildActor` (`self.BP_ViewWindow3`))))
      (bind _output_get_3 (set `self.EndTip` _asbp_view_window_4))
      (`/Game/Blueprints/BP_ViewWindow.ChangeVisibility` _output_get_3 false))))

(fn `StartTips`
  (`self.Event StartTips`))

(fn `UserConstructionScript`)