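; Waypoint trigger box that makes a BP_MIG jet fire projectiles when it flies into it.
; On overlap by anything other than BP_Projectile or BP_Unkers, StartFiring casts the actor's parent to BP_MIG and spawns BP_Projectile at its left, right and center guns.
; The NotActivated flag and a short Delay act as a re-trigger cooldown.
; ChangeSpeedOfJet, which scales JetSpeed, is defined but not called here.
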(event `self.ReceiveActorBeginOverlap`
  (params (OtherActor :type "Actor Object Reference"))
  (bind _returnvalue (`GameplayStatics.GetObjectClass` OtherActor))
  (if (or (== _returnvalue "/Game/Blueprints/Waypoint_System/BP_Projectile.BP_Projectile_C") (== _returnvalue "/Game/Blueprints/BP_Unkers.BP_Unkers_C"))
    _
    (elif (`self.NotActivated`)
      (`self.StartFiring` OtherActor)
      (set `self.NotActivated` false)
      (`KismetSystemLibrary.Delay` 3.0)
      (set `self.NotActivated` true))))

(fn `ChangeSpeedOfJet`
  (params (`In Actor` :type "Actor Object Reference") (Multiplier :type "Float (double-precision)"))
  (bind _asbp_mig (cast `/Game/Blueprints/BP_MIG` (`self.GetParentActor` `In Actor`)))
  (set `/Game/Blueprints/BP_MIG.JetSpeed` (* (`/Game/Blueprints/BP_MIG.JetSpeed` _asbp_mig) Multiplier) _asbp_mig)
  (set `self.NotActivated` false))

(fn `StartFiring`
  (params (`In Actor` :type "Actor Object Reference"))
  (bind _asbp_mig (cast `/Game/Blueprints/BP_MIG` (`self.GetParentActor` `In Actor`))
    (:`then`
      (`|ExecutionSequence`
        (:`then_0`
          (bind _gunleft (`/Game/Blueprints/BP_MIG.GunLeft` _asbp_mig))
          (`|SpawnActorFromClass` "/Game/Blueprints/Waypoint_System/BP_Projectile.BP_Projectile_C" (`KismetMathLibrary.MakeTransform` (`SceneComponent.K2_GetComponentLocation` _gunleft) (`SceneComponent.K2_GetComponentRotation` _gunleft)) "Undefined" "MultiplyWithRoot" null null))
        (:`then_1`
          (bind _gunright (`/Game/Blueprints/BP_MIG.GunRight` _asbp_mig))
          (`|SpawnActorFromClass` "/Game/Blueprints/Waypoint_System/BP_Projectile.BP_Projectile_C" (`KismetMathLibrary.MakeTransform` (`SceneComponent.K2_GetComponentLocation` _gunright) (`SceneComponent.K2_GetComponentRotation` _gunright)) "Undefined" "MultiplyWithRoot" null null))
        (:`then_2`
          (bind _guncenter (`/Game/Blueprints/BP_MIG.GunCenter` _asbp_mig))
          (`|SpawnActorFromClass` "/Game/Blueprints/Waypoint_System/BP_Projectile.BP_Projectile_C" (`KismetMathLibrary.MakeTransform` (`SceneComponent.K2_GetComponentLocation` _guncenter) (`SceneComponent.K2_GetComponentRotation` _guncenter)) "Undefined" "MultiplyWithRoot" null null))))
    (:`CastFailed`
      (`KismetSystemLibrary.PrintString` "Hello"))))

(fn `UserConstructionScript`)