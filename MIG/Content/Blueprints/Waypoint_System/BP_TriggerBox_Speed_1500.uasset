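; BP_TriggerBox_Speed_1500 is a waypoint-system trigger that ramps up the speed of a BP_MIG jet passing through it.
; On overlap it casts the other actor's parent to BP_MIG, then loops through a Delay, adding a fixed JetSpeed step via ChangeSpeedOfJet until SpeedToSet is reached.
; NotActivated gates re-entry: a parallel sequence branch re-arms it after a delay, though each speed step clears it again.
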(event `self.ReceiveActorBeginOverlap`
  (params (OtherActor :type "Actor Object Reference"))
  (`|ExecutionSequence`
    (:`then_0`
      (if (`self.NotActivated`)
        (set `self.NotActivated` false)
        (bind _asbp_mig (cast `/Game/Blueprints/BP_MIG` (`self.GetParentActor` OtherActor)))
        (if (< (`/Game/Blueprints/BP_MIG.JetSpeed` _asbp_mig) (`self.Speed To Set`)) :!label _label
          (`KismetSystemLibrary.Delay` 0.3)
          (`self.ChangeSpeedOfJet` OtherActor :!pinned true) ; Изменяет скорость самолета на множитель Multiplier\nДля работы подсоединить свойство Other Actor к In Actor
          (goto _label))))
    (:`then_1`
      (`KismetSystemLibrary.Delay` 3.0)
      (set `self.NotActivated` true))))

(fn `ChangeSpeedOfJet`
  (params (`In Actor` :type "Actor Object Reference"))
  (bind _asbp_mig (cast `/Game/Blueprints/BP_MIG` (`self.GetParentActor` `In Actor`)))
  (set `/Game/Blueprints/BP_MIG.JetSpeed` (+ (`/Game/Blueprints/BP_MIG.JetSpeed` _asbp_mig) 100.0) _asbp_mig)
  (set `self.NotActivated` false))

(fn `UserConstructionScript`)