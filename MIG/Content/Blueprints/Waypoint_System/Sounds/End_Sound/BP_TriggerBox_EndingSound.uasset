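; BP_TriggerBox_EndingSound is a trigger in the waypoint system that fades the MIG jet's passive flight sound in and out.
; A BP_ViewWindow entering StartCube fades in the parent BP_MIG's MIGFlyPassive and clears NotActivated, so this fires only once.
; With that flag cleared, leaving EndCube fades the sound out more slowly.
; An unreferenced ChangeSpeedOfJet function raises JetSpeed and clears the same flag.
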(event `self.StartCube.OnComponentBeginOverlap`
  (params (OverlappedComponent :type "PrimitiveComponent Object Reference") (OtherActor :type "Actor Object Reference") (OtherComp :type "PrimitiveComponent Object Reference") (OtherBodyIndex :type Integer) (bFromSweep :type Boolean) (SweepResult :type "HitResult Structure (by ref)"))
  (if (== (`GameplayStatics.GetObjectClass` OtherActor) "/Game/Blueprints/Waypoint_System/BP_Projectile.BP_Projectile_C")
    _
    (elif (and (== (`GameplayStatics.GetObjectClass` OtherActor) "/Game/Blueprints/BP_ViewWindow.BP_ViewWindow_C") (`self.NotActivated`))
      (set `self.NotActivated` false)
      (bind _asbp_mig (cast `/Game/Blueprints/BP_MIG` (`self.GetParentActor` OtherActor)))
      (`AudioComponent.FadeIn` (`/Game/Blueprints/BP_MIG.MIG_fly_passive` _asbp_mig) 2.0 1.0 0.0 "Linear"))))

(event `self.EndCube.OnComponentEndOverlap`
  (params (OverlappedComponent :type "PrimitiveComponent Object Reference") (OtherActor :type "Actor Object Reference") (OtherComp :type "PrimitiveComponent Object Reference") (OtherBodyIndex :type Integer))
  (if (== (`GameplayStatics.GetObjectClass` OtherActor) "/Game/Blueprints/Waypoint_System/BP_Projectile.BP_Projectile_C")
    _
    (elif (and (== (`GameplayStatics.GetObjectClass` OtherActor) "/Game/Blueprints/BP_ViewWindow.BP_ViewWindow_C") (!= (`self.NotActivated`) true))
      (set `self.NotActivated` false)
      (bind _asbp_mig (cast `/Game/Blueprints/BP_MIG` (`self.GetParentActor` OtherActor)))
      (`AudioComponent.FadeOut` (`/Game/Blueprints/BP_MIG.MIG_fly_passive` _asbp_mig) 5.0 0.0 "Linear"))))

(fn `ChangeSpeedOfJet`
  (params (`In Actor` :type "Actor Object Reference"))
  (bind _asbp_mig (cast `/Game/Blueprints/BP_MIG` (`self.GetParentActor` `In Actor`)))
  (set `/Game/Blueprints/BP_MIG.JetSpeed` (+ (`/Game/Blueprints/BP_MIG.JetSpeed` _asbp_mig) 100.0) _asbp_mig)
  (set `self.NotActivated` false))

(fn `UserConstructionScript`)