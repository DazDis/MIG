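; Waypoint-system trigger box that plays a one-shot 2D sound when a BP_ViewWindow actor overlaps it.
; The overlap checks for that exact class and clears the NotActivated flag so SoundToPlay fires only once.
; A ChangeSpeedOfJet function, not called within this Blueprint, raises the JetSpeed of a BP_MIG parent actor and clears the same flag.
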(event `self.ReceiveActorBeginOverlap`
  (params (OtherActor :type "Actor Object Reference"))
  (if (and (== (`GameplayStatics.GetObjectClass` OtherActor) "/Game/Blueprints/BP_ViewWindow.BP_ViewWindow_C") (`self.NotActivated`))
    (set `self.NotActivated` false)
    (`GameplayStatics.PlaySound2D` (`self.Sound To Play`) 1.0 1.0 0.0 null null)))

(fn `ChangeSpeedOfJet`
  (params (`In Actor` :type "Actor Object Reference"))
  (bind _asbp_mig (cast `/Game/Blueprints/BP_MIG` (`self.GetParentActor` `In Actor`)))
  (set `/Game/Blueprints/BP_MIG.JetSpeed` (+ (`/Game/Blueprints/BP_MIG.JetSpeed` _asbp_mig) 100.0) _asbp_mig)
  (set `self.NotActivated` false))

(fn `UserConstructionScript`)