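; Waypoint-system trigger box that switches on a timed fight phase for a spline-driven actor entering it.
; On overlap, while NotActivated is set, it finds BP_Spline two parent-actor levels above the overlapping actor and holds its FightOn true for five seconds.
; A separate ChangeSpeedOfJet function raises a parent BP_MIG's JetSpeed and clears NotActivated, but the event graph never calls it.
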(event `self.ReceiveActorBeginOverlap`
  (params (OtherActor :type "Actor Object Reference"))
  (if (`self.NotActivated`)
    (bind _asbp_spline (cast `/Game/Blueprints/Waypoint_System/BP_Spline` (`self.GetParentActor` (`self.GetParentActor` OtherActor))))
    (set `/Game/Blueprints/Waypoint_System/BP_Spline.FightOn` true _asbp_spline)
    (`KismetSystemLibrary.Delay` 5.0)
    (set `/Game/Blueprints/Waypoint_System/BP_Spline.FightOn` false _asbp_spline)))

(fn `ChangeSpeedOfJet`
  (params (`In Actor` :type "Actor Object Reference"))
  (bind _asbp_mig (cast `/Game/Blueprints/BP_MIG` (`self.GetParentActor` `In Actor`)))
  (set `/Game/Blueprints/BP_MIG.JetSpeed` (+ (`/Game/Blueprints/BP_MIG.JetSpeed` _asbp_mig) 100.0) _asbp_mig)
  (set `self.NotActivated` false))

(fn `UserConstructionScript`)